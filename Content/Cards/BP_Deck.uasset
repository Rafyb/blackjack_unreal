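; BP_Deck is an actor that builds a shuffled playing-card deck and spawns it as a stack of BP_Card actors when play begins.
; GenerateDeck pairs four suits with ranks from Ace to King as card structs, then shuffles the array.
; BeginPlay spawns a card per struct, passing in suit and value and using each new card's root as the next spawn anchor, one unit higher.
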(event EventBeginPlay
  (Variables|Default|SetSpawn%20Location (Variables|Default|GetDefaultSceneRoot))
  (CallFunction|GenerateDeck)
  (for _array_element (Variables|Default|GetCard%20Deck%20Array)
    (bind _returnvalue (Game|SpawnActorfromClass "/Game/Cards/BP_Card.BP_Card_C" (Math|Transform|MakeTransform (+ (Transformation|GetWorldLocation (Variables|Default|GetSpawn%20Location)) "0,0.000000,1.000000") "0, 0, 0" "1,1,1") "Undefined" 0 (.suit _array_element) (Utilities|Text|ToText(String) (.value _array_element)) 0))
    (Variables|Default|SetSpawn%20Location (Variables|/Game/Cards/BP_Card.BP_Card_C|GetDefaultSceneRoot _returnvalue))))

(fn ConstructionScript)

(fn GenerateDeck
  (bind _card_suit_index (LocalVariables|GetCard%20Suit%20Index))
  (LocalVariables|SetSuit%20Array (Utilities|Array|MakeArray "/Game/Textures/heart.heart" "/Game/Textures/clubb.clubb" "/Game/Textures/spade.spade" "/Game/Textures/diamond.diamond"))
  (LocalVariables|SetCard%20Value%20Array (Utilities|Array|MakeArray "A" "2" "3" "4" "5" "6" "7" "8" "9" "10" "J" "Q" "K"))
  (while (< (LocalVariables|GetCard%20Index) (LocalVariables|GetCount)) :!label _label
    (bind _structout (Utilities|Struct|SetmembersinBP_MyCardStruct (LocalVariables|GetNew%20Card) (Utilities|Array|Get(acopy) (LocalVariables|GetSuit%20Array) (LocalVariables|GetCard%20Suit%20Index)) (Utilities|Array|Get(acopy) (LocalVariables|GetCard%20Value%20Array) (LocalVariables|GetCard%20Index))))
    (Utilities|Array|Add (Variables|Default|GetCard%20Deck%20Array) _structout)
    (Math|Integer|IncrementInt (LocalVariables|GetCard%20Index)))
  (Math|Integer|IncrementInt _card_suit_index
    (:%20%20
      (if (< _card_suit_index 4)
        (LocalVariables|SetCard%20Index 0)
        (goto _label)
        (else
          (Utilities|Array|Shuffle (Variables|Default|GetCard%20Deck%20Array)))))))